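; Puzzle event component that runs entry into and exit from puzzle mode for its RXPuzzelBase owner.
; BeginPlay caches the fade widget, Nowiniq spawn manager, start tile and puzzle-specific end tile.
; Start and end swap input mappings, fade and call C++ parents, with start briefly locking input and lighting tiles.
; End destroys tiles, finishes the puzzle and spawns Nowiniq; without a start tile (Temple puzzle), it only finishes.
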(event Custom|DisablePlayerInput
  (bind _returnvalue (Game|Player|GetPlayerPawn 0))
  (bind _returnvalue_2 (Game|GetPlayerController 0))
  (Input|DisableInput _returnvalue _returnvalue_2)
  (Utilities|FlowControl|Delay 1.5)
  (Input|EnableInput _returnvalue _returnvalue_2))

(event EventBeginPlay
  ;[1 1 1] 쓰일 변수들 초기화 페이드위젯, 타일들
  (bind _returnvalue (UserInterface|CreateWidget "/Game/UI/WBP_FadeAnimWidget.WBP_FadeAnimWidget_C"))
  (Variables|Default|SetFadeWiget _returnvalue)
  (bind _returnvalue_2 (Actor|GetActorOfClass "/Game/Blueprints/Puzzel/BP_PuzzelNowiniqSpawnManager.BP_PuzzelNowiniqSpawnManager_C"))
  (Variables|Default|SetNowiniqSpawnManager _returnvalue_2)
  (bind _returnvalue_3 (Actor|GetActorOfClass "/Game/Blueprints/Puzzel/BP_Puzzel_StartTile.BP_Puzzel_StartTile_C"))
  (bind _output_get (Variables|Default|SetPuzzelStartTile _returnvalue_3))
  (Utilities|IsValid _output_get
    (:Is%20Valid
      (bind _asrxpuzzel_base (Utilities|Casting|CastToRXPuzzelBase (Components|GetOwner)))
      ;[1 1 1] 퍼즐에 맞는 EndTile을 가져와서 저장하는 로직
      (switch name (Class|RXPuzzelBase|GetPuzzelName _asrxpuzzel_base)
        (:EulerPuzzel
          (bind _returnvalue_4 (Actor|GetActorOfClass "/Game/Blueprints/Puzzel/EulerPuzzel/BP_Puzzel_EulerEndTile.BP_Puzzel_EulerEndTile_C"))
          (Variables|Default|SetEulerPuzzelEndTile _returnvalue_4))
        (:BlindPuzzel
          (bind _returnvalue_5 (Actor|GetActorOfClass "/Game/Blueprints/Puzzel/BlindPuzzel/BP_Puzzel_BlindEndTile.BP_Puzzel_BlindEndTile_C"))
          (Variables|Default|SetBlindPuzzelEndTile _returnvalue_5))
        (:PushablePuzzel
          (bind _returnvalue_6 (Actor|GetActorOfClass "/Game/Blueprints/Puzzel/PushablePuzzel/BP_Puzzel_PushableEndTile.BP_Puzzel_PushableEndTile_C"))
          (Variables|Default|SetPushablePuzzelEndTile _returnvalue_6))
        (:PatternPuzzel
          (bind _returnvalue_7 (Actor|GetActorOfClass "/Game/Blueprints/Puzzel/PatternPuzzel/BP_Puzzel_PatternEndTile.BP_Puzzel_PatternEndTile_C"))
          (Variables|Default|SetPatternPuzzelEndTile _returnvalue_7))
        (:TimingPuzzel
          (bind _returnvalue_8 (Actor|GetActorOfClass "/Game/Blueprints/Puzzel/TimingPuzzel/BP_Puzzel_TimingEndTile.BP_Puzzel_TimingEndTile_C"))
          (Variables|Default|SetTimingPuzzelEndTile _returnvalue_8))))))

(event EventStartPuzzelMode
  (bind _fadewiget (Variables|Default|GetFadeWiget))
  (bind _eulerpuzzelendtile (Variables|Default|GetEulerPuzzelEndTile))
  (bind _timingpuzzelendtile (Variables|Default|GetTimingPuzzelEndTile))
  (bind _blindpuzzelendtile (Variables|Default|GetBlindPuzzelEndTile))
  (bind _patternpuzzelendtile (Variables|Default|GetPatternPuzzelEndTile))
  (bind _pushablepuzzelendtile (Variables|Default|GetPushablePuzzelEndTile))
  (bind _puzzelstarttile (Variables|Default|GetPuzzelStartTile))
  ;[1 1 1] 퍼즐모드 시작 : BlueprintNativeEvent
  (bind _asrxplayer_controller (Utilities|Casting|CastToRXPlayerController (Game|GetPlayerController 0)))
  ;[1 1 1] 컨트롤러 퍼즐전용으로 교체
  (Input|RemoveMappingContext (PlayerController|LocalPlayerSubsystems|GetEnhancedInputLocalPlayerSubsystem _asrxplayer_controller) "/Game/Input/IMC_Default.IMC_Default" "(bIgnoreAllPressedKeysUntilRelease=True,bForceImmediately=False,bNotifyUserSettings=False)")
  (Input|AddMappingContext (PlayerController|LocalPlayerSubsystems|GetEnhancedInputLocalPlayerSubsystem _asrxplayer_controller) "/Game/Input/IMC_Puzzel.IMC_Puzzel" 0 "(bIgnoreAllPressedKeysUntilRelease=True,bForceImmediately=False,bNotifyUserSettings=False)")
  ;[1 1 1] 페이드이벤트발생
  (UserInterface|Viewport|AddtoViewport _fadewiget 0)
  (Default|PlayFadeOut _fadewiget)
  ;[1 1 1] CPP 부모호출 : 카메라셋팅, 플레이어 퍼즐이벤트 진입
  (|CallParentFunction)
  (Audio|PlaySound2D "/Game/Audio/SFX/Puzzel/SFX_Puzzle_Interaction.SFX_Puzzle_Interaction" 1.0 1.0 0.0 0 0)
  ;[1 1 1] 퍼즐이벤트 시작 : 인풋 1.5 정지 후, 퍼즐시작, 종료타일 색 활성화
  (CallFunction|DisablePlayerInput)
  (Utilities|IsValid _puzzelstarttile
    (:Is%20Valid
      (Default|SetActiveColor _puzzelstarttile)
      (Utilities|FlowControl|Sequence
        (:then_0
          (Utilities|IsValid _eulerpuzzelendtile
            (:Is%20Valid
              (Default|SetActiveColor _eulerpuzzelendtile))))
        (:then_1
          (Utilities|IsValid _blindpuzzelendtile
            (:Is%20Valid
              (Default|SetActiveColor _blindpuzzelendtile))))
        (:then_2
          (Utilities|IsValid _pushablepuzzelendtile
            (:Is%20Valid
              (Default|SetActiveColor _pushablepuzzelendtile))))
        (:then_3
          (Utilities|IsValid _patternpuzzelendtile
            (:Is%20Valid
              (Default|SetActiveColor _patternpuzzelendtile))))
        (:then_4
          (Utilities|IsValid _timingpuzzelendtile
            (:Is%20Valid
              (Default|SetActiveColor _timingpuzzelendtile))))))))

(event EventEndPuzzelMode
  (bind _fadewiget (Variables|Default|GetFadeWiget))
  (bind _patternpuzzelendtile (Variables|Default|GetPatternPuzzelEndTile))
  (bind _timingpuzzelendtile (Variables|Default|GetTimingPuzzelEndTile))
  (bind _puzzelstarttile (Variables|Default|GetPuzzelStartTile))
  (bind _pushablepuzzelendtile (Variables|Default|GetPushablePuzzelEndTile))
  (bind _eulerpuzzelendtile (Variables|Default|GetEulerPuzzelEndTile))
  (bind _blindpuzzelendtile (Variables|Default|GetBlindPuzzelEndTile))
  ;[1 1 1] 퍼즐모드 해제 : BlueprintNativeEvent
  (bind _asrxplayer_controller (Utilities|Casting|CastToRXPlayerController (Game|GetPlayerController 0)))
  (Input|RemoveMappingContext (PlayerController|LocalPlayerSubsystems|GetEnhancedInputLocalPlayerSubsystem _asrxplayer_controller) "/Game/Input/IMC_Puzzel.IMC_Puzzel" "(bIgnoreAllPressedKeysUntilRelease=True,bForceImmediately=False,bNotifyUserSettings=False)")
  (Input|AddMappingContext (PlayerController|LocalPlayerSubsystems|GetEnhancedInputLocalPlayerSubsystem _asrxplayer_controller) "/Game/Input/IMC_Default.IMC_Default" 0 "(bIgnoreAllPressedKeysUntilRelease=True,bForceImmediately=False,bNotifyUserSettings=False)")
  (UserInterface|Viewport|AddtoViewport _fadewiget 0)
  (Default|PlayFadeOut _fadewiget)
  ;[1 1 1] CPP 부모호출 : 카메라셋팅, 플레이어 퍼즐이벤트 진입해제
  (|CallParentFunction)
  (Utilities|IsValid _puzzelstarttile
    (:Is%20Valid
      ;[1 1 1] 퍼즐이벤트 종료 : 퍼즐시작, 종료타일 삭제, 퍼즐컴포넌트 삭제
      (Actor|DestroyActor _puzzelstarttile)
      (Utilities|FlowControl|Sequence
        (:then_0
          (Utilities|IsValid _eulerpuzzelendtile
            (:Is%20Valid
              (Actor|DestroyActor _eulerpuzzelendtile))))
        (:then_1
          (Utilities|IsValid _blindpuzzelendtile
            (:Is%20Valid
              (Actor|DestroyActor _blindpuzzelendtile))))
        (:then_2
          (Utilities|IsValid _pushablepuzzelendtile
            (:Is%20Valid
              (Actor|DestroyActor _pushablepuzzelendtile))))
        (:then_3
          (Utilities|IsValid _patternpuzzelendtile
            (:Is%20Valid
              (Actor|DestroyActor _patternpuzzelendtile))))
        (:then_4
          (Utilities|IsValid _timingpuzzelendtile
            (:Is%20Valid
              (Actor|DestroyActor _timingpuzzelendtile)))))
      (bind _asbp_puzzel_parent (Utilities|Casting|CastToBP_Puzzel_Parent (Components|GetOwner)))
      (Class|RXPuzzelBase|PuzzelEventFinish _asbp_puzzel_parent)
      ;[1 1 1] 퍼즐 클리어 시 노이닉 스폰
      (bind _asrxpuzzel_base (Utilities|Casting|CastToRXPuzzelBase (Components|GetOwner)))
      (Default|SpawnNowiniq (Variables|Default|GetNowiniqSpawnManager) (Class|RXPuzzelBase|GetPuzzelName _asrxpuzzel_base))
      (Audio|PlaySound2D "/Game/Audio/SFX/Puzzel/SFX_PuzzleSolvedSound.SFX_PuzzleSolvedSound" 1.0 1.0 0.0 0 0))
    (:Is%20Not%20Valid
      ;[1 1 1] TemplePuzzel 전용 플로우(TemplePuzzel->NotUseStartTile)
      (bind _asrxpuzzel_base_2 (Utilities|Casting|CastToRXPuzzelBase (Components|GetOwner)))
      (Class|RXPuzzelBase|PuzzelEventFinish _asrxpuzzel_base_2))))